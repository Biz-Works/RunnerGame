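; BP_Coin_BLue is a blue coin pickup that is worth five coins to the player.
; On actor overlap it casts the other actor to BP_PlayerCharacter and, on success, adds the value directly to that character's CoinCount.
; It then plays a sound at the player's location and destroys itself.
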(event EventBeginPlay
  (|CallParentFunction) ; This node is disabled and will not be called.\nDrag off pins to build functionality.
)

(event Collision|EventActorBeginOverlap
  (params (OtherActor :type Actor%20Object%20Reference))
  (bind _asbp_player_character (Utilities|Casting|CastToBP_PlayerCharacter OtherActor))
  (Variables|/Game/ThirdPerson/Blueprints/BP_PlayerCharacter.BP_PlayerCharacter_C|SetCoinCount _asbp_player_character (+ (Variables|/Game/ThirdPerson/Blueprints/BP_PlayerCharacter.BP_PlayerCharacter_C|GetCoinCount _asbp_player_character) 5))
  (Audio|PlaySoundatLocation (Variables|Default|GetSound) (Transformation|GetActorLocation _asbp_player_character) "0, 0, 0" 1.0 1.0 0.0 0 0 0 0)
  (Actor|DestroyActor))

(fn ConstructionScript
  (|CallParentFunction))