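; Bush obstacle that temporarily slows the player character when it enters the bush's Box trigger.
; After a negative-duration Delay, the overlap casts to BP_PlayerCharacter, caches BaseWalkSpeed and divides it by WalkSpeedDivide.
; After SlowDuration it restores the cached speed, whether or not the player has left the box.
; A re-overlap during the slow overwrites the cache with the already reduced speed.
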(event OnComponentBeginOverlap(Box)
  (params (OverlappedComponent :type Primitive%20Component%20Object%20Reference) (OtherActor :type Actor%20Object%20Reference) (OtherComp :type Primitive%20Component%20Object%20Reference) (OtherBodyIndex :type Integer) (bFromSweep :type Boolean) (SweepResult :type Hit%20Result%20Structure%20%28by%20ref%29))
  (Utilities|FlowControl|Delay -1e+01)
  (bind _asbp_player_character (Utilities|Casting|CastToBP_PlayerCharacter OtherActor)
    (:then
      (Variables|Default|SetCachedWalkSpeed (Variables|/Game/ThirdPerson/Blueprints/BP_PlayerCharacter.BP_PlayerCharacter_C|GetBaseWalkSpeed _asbp_player_character))
      (Variables|/Game/ThirdPerson/Blueprints/BP_PlayerCharacter.BP_PlayerCharacter_C|SetBaseWalkSpeed _asbp_player_character (Math|Float|SafeDivide (Variables|/Game/ThirdPerson/Blueprints/BP_PlayerCharacter.BP_PlayerCharacter_C|GetBaseWalkSpeed _asbp_player_character) (Variables|Default|GetWalkSpeedDivide)))
      (Utilities|FlowControl|Delay (Variables|Default|GetSlowDuration))
      (Variables|/Game/ThirdPerson/Blueprints/BP_PlayerCharacter.BP_PlayerCharacter_C|SetBaseWalkSpeed _asbp_player_character (Variables|Default|GetCachedWalkSpeed)))
    (:CastFailed
      (Development|PrintString "CAST FAILED" true true "(R=1.000000,G=0.016322,B=0.000000,A=1.000000)" 5.0))))

(event EventBeginPlay)

(event Collision|EventActorBeginOverlap
  (params (OtherActor :type Actor%20Object%20Reference)))

(event EventTick
  (params (DeltaSeconds :type Float%20%28single-precision%29)))

(fn ConstructionScript)